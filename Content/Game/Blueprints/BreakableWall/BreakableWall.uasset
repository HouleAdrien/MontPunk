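; Breakable wall actor that shatters when hit while at least three BP_SBIRE pawns are crowded around it.
; On a StaticMesh hit, a box overlap at the actor location counts those pawns.
; At the threshold it destroys the mesh, adds a geometry collection component in its place and scatters it with a radial impulse.
; The whole actor is destroyed after a short delay.
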(event `self.ReceiveBeginPlay`)

(event `self.StaticMesh.OnComponentHit`
  (params (HitComponent :type "PrimitiveComponent Object Reference") (OtherActor :type "Actor Object Reference") (OtherComp :type "PrimitiveComponent Object Reference") (NormalImpulse :type "Vector Structure") (Hit :type "HitResult Structure (by ref)"))
  (bind _outactors (`KismetSystemLibrary.BoxOverlapActors` (`self.K2_GetActorLocation`) (50.0 100.0 100.0) (`|MakeArray` "ObjectTypeQuery3" :!type "EObjectTypeQuery Enum") "/Game/Game/Blueprints/Sbire/BP_SBIRE.BP_SBIRE_C"))
  (if (>= (`KismetArrayLibrary.Array_Length` _outactors) 3)
    (`ActorComponent.K2_DestroyComponent` (`self.StaticMesh`))
    (bind _returnvalue (`AddComponent|NODE_AddGeometryCollectionComponent-0`))
    (`PrimitiveComponent.AddRadialImpulse` _returnvalue (`self.K2_GetActorLocation`) 100.0 250000.0 "RIF_Constant" false)
    (`KismetSystemLibrary.Delay` 5.0)
    (`self.K2_DestroyActor`)))

(fn `UserConstructionScript`)