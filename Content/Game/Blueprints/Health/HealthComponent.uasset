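; HealthComponent tracks an entity's health, starting at MaxHealth, and handles damage and healing events.
; Damage is ignored during brief invincibility frames, which each non-lethal hit starts and Tick counts down.
; Lethal damage reloads the current level for the player and has no further effect for other entities.
; Healing takes the larger of MaxHealth and the healed total, so it never caps health, and prints the result.
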(event `self.ReceiveBeginPlay`
  (set `self.currentHealth` (`self.maxHealth`)))

(event `DealDamageEvent`
  (params (Damage :type "Float (double-precision)"))
  ;[1 1 1] Deal Damage to entity
  (if (not (`self.isInvicible`))
    (bind _isdead (`self.takeDamage` Damage))
    (if _isdead
      (if (`self.isPlayer`)
        (bind _returnvalue (`GameplayStatics.GetCurrentLevelName` true))
        (`GameplayStatics.OpenLevel` (`KismetStringLibrary.Conv_StringToName` _returnvalue)))
      (else
        (set `self.invicibilityDuration` 0.2)
        (set `self.isInvicible` true)))))

(event `self.ReceiveTick`
  (params (DeltaSeconds :type "Float (single-precision)"))
  ;[1 1 1] Update invicibility frames
  (bind _output_get (set `self.invicibilityDuration` (- (`self.invicibilityDuration`) DeltaSeconds)))
  (set `self.isInvicible` (> _output_get 0.0)))

(event `HealEvents`
  (params (HealAmount :type "Float (double-precision)"))
  ;[1 1 1] Heal event
  (`self.heal` HealAmount))

(fn `heal`
  (params (HealAmount :type "Float (double-precision)"))
  (bind _output_get (set `self.currentHealth` (`KismetMathLibrary.FMax` (`self.maxHealth`) (+ HealAmount (`self.currentHealth`)))))
  (`KismetSystemLibrary.PrintString` (`KismetStringLibrary.Conv_DoubleToString` _output_get)))

(fn `takeDamage`
  (params (Damage :type "Float (double-precision)"))
  (returns (IsDead :type Boolean))
  (bind _output_get (set `self.currentHealth` (- (`self.currentHealth`) Damage)))
  (return (<= _output_get 0.0)))