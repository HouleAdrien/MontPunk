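; Boss enemy actor that chases and attacks the player, with a health bar that turns toward the camera.
; Pawn sensing starts a timed focus on the player, while Tick feeds sight and close-range flags to the AI blackboard.
; CloseATk faces the target, then after a delay deals sphere-overlap damage.
; A hit event with the player character drops random loot and destroys the boss, regardless of health.
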(event `self.ReceiveTick`
  (params (DeltaSeconds :type "Float (single-precision)"))
  (bind _healthcomponent (`self.HealthComponent`))
  (bind _healthbar (`self.HealthBar`))
  (bind _returnvalue (`AIBlueprintHelperLibrary.GetBlackboard` (`AIBlueprintHelperLibrary.GetAIController` self)))
  (bind _returnvalue_2 (/ (`/Game/Game/Blueprints/Health/HealthComponent.currentHealth` _healthcomponent) (`/Game/Game/Blueprints/Health/HealthComponent.maxHealth` _healthcomponent)))
  (bind _returnvalue_3 (<= (`self.GetDistanceTo` self (`self.target`)) (`self.closeRangeAttackDistance`)))
  (set `/Game/Game/Blueprints/Health/HealthComponent.isPlayer` false (`self.HealthComponent`))
  ;[1 1 1] Health Bar update
  (if (not (== (`self.Previous Percent`) _returnvalue_2))
    (bind _asennemy_health_bar (cast `/Game/Game/Blueprints/UI/EnnemyHealthBar` (`WidgetComponent.GetWidget` (`self.HealthBar`))))
    (bind _output_get (set `self.Previous Percent` _returnvalue_2))
    (`ProgressBar.SetPercent` (`/Game/Game/Blueprints/UI/EnnemyHealthBar.HealthBar` _asennemy_health_bar) _output_get))
  (`SceneComponent.K2_SetWorldRotation` _healthbar (`KismetMathLibrary.FindLookAtRotation` (`SceneComponent.K2_GetComponentLocation` _healthbar) (`SceneComponent.K2_GetComponentLocation` (`Actor.RootComponent` (`GameplayStatics.GetPlayerCameraManager` 0)))) false false)
  ;[1 1 1] Chase And Attack Logic
  (if (`self.following`)
    (bind _output_get_2 (set `self.focusTimer` (- (`self.focusTimer`) DeltaSeconds)))
    (if (<= _output_get_2 0.0)
      (set `self.following` false)
      (`BlackboardComponent.SetValueAsBool` _returnvalue "HasSeenPlayer?" false)
      (else
        (`BlackboardComponent.SetValueAsBool` _returnvalue "IsInCloseRange?" _returnvalue_3)
        (set `self.hasEnnemyIncloseRange` _returnvalue_3)))))

(event `self.PawnSensing.OnSeePawn`
  (params (Pawn :type "Pawn Object Reference"))
  (cast `/Game/Game/Blueprints/BP_ThirdPersonCharacter` Pawn)
  (`BlackboardComponent.SetValueAsBool` (`AIBlueprintHelperLibrary.GetBlackboard` (`AIBlueprintHelperLibrary.GetAIController` self)) "HasSeenPlayer?" true)
  (set `self.focusTimer` 5.0)
  (set `self.following` true)
  (set `self.target` Pawn))

(event `self.ReceiveHit`
  (params (MyComp :type "PrimitiveComponent Object Reference") (Other :type "Actor Object Reference") (OtherComp :type "PrimitiveComponent Object Reference") (bSelfMoved :type Boolean) (HitLocation :type "Vector Structure") (HitNormal :type "Vector Structure") (NormalImpulse :type "Vector Structure") (Hit :type "HitResult Structure (by ref)"))
  (cast `/Game/Game/Blueprints/BP_ThirdPersonCharacter` Other)
  (for _ (range (+ (`KismetMathLibrary.RandomInteger` 5) 1))
    (`/Game/Game/Blueprints/Money/AI_LootDrop.DropLoot` (`self.AI_LootDrop`) self))
  (`self.K2_DestroyActor`))

(event `CloseATk`
  (bind _target (`self.target`))
  (bind (_returnvalue_roll _returnvalue_pitch _returnvalue_yaw) (`KismetMathLibrary.BreakRotator` (`KismetMathLibrary.FindLookAtRotation` (`self.K2_GetActorLocation`) (`self.K2_GetActorLocation` _target))))
  ;[1 1 1] AtkClose
  (`|ExecutionSequence`
    (:`then_0`
      (`/Engine/EditorBlueprintResources/StandardMacros.IsValid` _target
        (:`Is Valid`
          (`self.K2_SetActorRotation` (`KismetMathLibrary.MakeRotator` 0.0 0.0 _returnvalue_yaw)))))
    (:`then_1`
      (`KismetSystemLibrary.Delay` 1.0)
      (bind _outactors (`KismetSystemLibrary.SphereOverlapActors` (`self.K2_GetActorLocation`) (`self.closeRangeAttackDistance`) (`|MakeArray` "ObjectTypeQuery3" :!type "EObjectTypeQuery Enum")))
      (for _array_element _outactors
        (bind _asbp_third_person_character (cast `/Game/Game/Blueprints/BP_ThirdPersonCharacter` _array_element))
        (`/Game/Game/Blueprints/Health/HealthComponent.DealDamageEvent` (`self.GetComponentByClass` _asbp_third_person_character "/Game/Game/Blueprints/Health/HealthComponent.HealthComponent_C") 3.0))
      (`BlackboardComponent.SetValueAsBool` (`AIBlueprintHelperLibrary.GetBlackboard` (`AIBlueprintHelperLibrary.GetAIController` self)) "IsInCloseRange?" false)
      (set `self.hasEnnemyIncloseRange` false))))

(fn `UserConstructionScript`)