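; Money Blueprint that tracks a current money value against a maximum and exposes it through a getter.
; Loot events add either one unit or a given amount via AddMoney, and RemoveMoney subtracts via ConsumeMoney.
; Both functions check the limit only before changing the value, without clamping, so a single change can overshoot the maximum or drop below zero.
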(event `LootMoney`
  (`self.AddMoney` 1))

(event `LootMoneyAmount`
  (params (Value :type Integer))
  (`self.AddMoney` Value))

(event `RemoveMoney`
  (params (Value :type Integer))
  (`self.ConsumeMoney` Value))

(fn `AddMoney`
  (params (Value :type Integer))
  (if (< (`self.CurrentValue`) (`self.MaxValue`))
    (set `self.CurrentValue` (+ Value (`self.CurrentValue`)))))

(fn `ConsumeMoney`
  (params (Value :type Integer))
  (if (> (`self.CurrentValue`) 0)
    (set `self.CurrentValue` (- (`self.CurrentValue`) Value))))

(fn `GetMoney`
  (returns (Value :type Integer))
  (return (`self.CurrentValue`)))