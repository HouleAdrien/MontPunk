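; Mutant spawner actor that periodically spawns a random enemy class inside a box zone while the player is within range.
; A delayed self-calling check spawns only while the world-wide count of the checked class is below a cap.
; Each spawn gets a random point and yaw, then a downward trace snaps it to the ground.
; A separate shut-off box, sized and placed by the construction script, pauses spawning while the player overlaps it.
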(event `SpawnCheck`
  (bind _spawnzone (`self.SpawnZone`))
  ;[1 1 1] SpawnZone
  (if (and (`self.active?`) (< (`self.GetDistanceTo` (`GameplayStatics.GetPlayerCharacter` 0)) (`self.PlayerLessThanDistance`))) :!label _label
    (bind _outactors (`GameplayStatics.GetAllActorsOfClass` (`self.EnemyTypeToCheck`)))
    (if (not (>= (`KismetArrayLibrary.Array_Length` _outactors) (`self.Enemy Amount`)))
      (bind _returnvalue (`|SpawnActorFromClass` (`KismetArrayLibrary.Array_Random` (`self.EnemyToSpawn`)) (`KismetMathLibrary.MakeTransform` (`KismetMathLibrary.RandomPointInBoundingBox` (`SceneComponent.K2_GetComponentLocation` _spawnzone) (`BoxComponent.GetScaledBoxExtent` _spawnzone)) (`KismetMathLibrary.MakeRotator` 0.0 0.0 (`KismetMathLibrary.RandomFloatInRange` -180.0 180.0))) "Undefined" "MultiplyWithRoot" null null))
      (`/Engine/EditorBlueprintResources/StandardMacros.IsValid` _returnvalue
        (:`Is Valid`
          (bind _output_get (set `self.Spawned Uit` _returnvalue))
          (bind _returnvalue_2 (`self.K2_GetActorLocation` _returnvalue))
          (bind (_outhit _returnvalue_3) (`KismetSystemLibrary.LineTraceSingle` _returnvalue_2 (- _returnvalue_2 (0.0 0.0 1000.0)) "TraceTypeQuery1" false (`|MakeArray` _output_get :!type "Actor Object Reference") "ForDuration"))
          (if _returnvalue_3
            (`self.K2_SetActorLocation` (`self.Spawned Uit`) (`.Location` (`GameplayStatics.BreakHitResult` _outhit)) false false)))
        (:`Is Not Valid`
          _))))
  (`KismetSystemLibrary.Delay` (`self.SpawnDelay`))
  (`self.SpawnCheck`))

(event `self.ReceiveBeginPlay`
  ;[1 1 1] SpawnZone
  (goto _label))

(event `self.ShutOffZone.OnComponentBeginOverlap`
  (params (OverlappedComponent :type "PrimitiveComponent Object Reference") (OtherActor :type "Actor Object Reference") (OtherComp :type "PrimitiveComponent Object Reference") (OtherBodyIndex :type Integer) (bFromSweep :type Boolean) (SweepResult :type "HitResult Structure (by ref)"))
  (cast `/Game/Game/Blueprints/BP_ThirdPersonCharacter` OtherActor)
  (set `self.active?` false))

(event `self.ShutOffZone.OnComponentEndOverlap`
  (params (OverlappedComponent :type "PrimitiveComponent Object Reference") (OtherActor :type "Actor Object Reference") (OtherComp :type "PrimitiveComponent Object Reference") (OtherBodyIndex :type Integer))
  (cast `/Game/Game/Blueprints/BP_ThirdPersonCharacter` OtherActor)
  (set `self.active?` true))

(fn `UserConstructionScript`
  (bind _shutoffzone (`self.ShutOffZone`))
  (`BoxComponent.SetBoxExtent` (`self.SpawnZone`) (`self.SpawnZoneSize`) true)
  (`BoxComponent.SetBoxExtent` _shutoffzone (`self.ShutOffZoneSize`) true)
  (`SceneComponent.K2_SetRelativeLocation` _shutoffzone (`self.ShutOffZoneLocation`) false false))