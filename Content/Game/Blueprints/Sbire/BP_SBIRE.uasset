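; BP_SBIRE is a robot minion that follows the player once seen via PawnSensing if IsFollowing is set, otherwise moves to PositionForRobots.
; BeginPlay increments the player's minion count up to four and assigns materials to the first three.
; The non-following Tick branch also updates the camera-facing health bar and destroys the minion at zero health, decrementing the count.
; LevelUpSkill increases its health, speed or damage level.
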(event `self.PawnSensing.OnSeePawn`
  (params (Pawn :type "Pawn Object Reference"))
  ;[1 1 1] Sbire movement
  (set `self.isSeingPlayer` true)
  (`self.FollowPlayer`))

(event `FollowPlayer`
  ;[1 1 1] Sbire movement
  (bind _returnvalue (`GameplayStatics.GetActorOfClass` "/Game/Game/Blueprints/BP_ThirdPersonCharacter.BP_ThirdPersonCharacter_C"))
  (if (`self.isSeingPlayer`)
    (if (`/Game/Game/Blueprints/BP_ThirdPersonCharacter.IsFollowing` _returnvalue)
      (`|AIMoveTo` self (0.0 0.0 0.0) (`GameplayStatics.GetPlayerCharacter` 0)))))

(event `self.ReceiveTick`
  (params (DeltaSeconds :type "Float (single-precision)"))
  (bind _healthbar (`self.HealthBar`))
  (bind _returnvalue (/ (`/Game/Game/Blueprints/Health/HealthComponent.currentHealth` (`self.HealthComponent`)) (`/Game/Game/Blueprints/Health/HealthComponent.maxHealth` (`self.HealthComponent`))))
  ;[1 1 1] Sbire movement
  (bind _returnvalue_2 (`GameplayStatics.GetActorOfClass` "/Game/Game/Blueprints/BP_ThirdPersonCharacter.BP_ThirdPersonCharacter_C"))
  (if (not (`/Game/Game/Blueprints/BP_ThirdPersonCharacter.IsFollowing` _returnvalue_2))
    (bind _returnvalue_3 (`GameplayStatics.GetActorOfClass` "/Game/Game/Blueprints/BP_ThirdPersonCharacter.BP_ThirdPersonCharacter_C"))
    (`|AIMoveTo` self (`/Game/Game/Blueprints/BP_ThirdPersonCharacter.PositionForRobots` _returnvalue_3) null
      (:`then`
        ;[1 1 1] Health Bar update
        (if (not (== (`self.previousPercent`) _returnvalue)) :!label _label
          (bind _aswb_health_bar (cast `/Game/Game/Blueprints/UI/WB_HealthBar` (`WidgetComponent.GetWidget` (`self.HealthBar`))))
          (bind _output_get (set `self.previousPercent` _returnvalue))
          (`ProgressBar.SetPercent` (`/Game/Game/Blueprints/UI/WB_HealthBar.HealthBar` _aswb_health_bar) _output_get))
        (`SceneComponent.K2_SetWorldRotation` _healthbar (`KismetMathLibrary.FindLookAtRotation` (`SceneComponent.K2_GetComponentLocation` _healthbar) (`SceneComponent.K2_GetComponentLocation` (`Actor.RootComponent` (`GameplayStatics.GetPlayerCameraManager` 0)))) false false)
        (if (<= (`/Game/Game/Blueprints/Health/HealthComponent.currentHealth` (`self.HealthComponent`)) 0.0)
          (`self.K2_DestroyActor`)
          (bind _returnvalue_4 (`GameplayStatics.GetActorOfClass` "/Game/Game/Blueprints/BP_ThirdPersonCharacter.BP_ThirdPersonCharacter_C"))
          (set `/Game/Game/Blueprints/BP_ThirdPersonCharacter.nbSbires` (- (`/Game/Game/Blueprints/BP_ThirdPersonCharacter.nbSbires` _returnvalue_4) 1) _returnvalue_4))))))

(event `self.ReceiveBeginPlay`
  (bind _mesh (`self.Mesh`))
  ;[1 1 1] Set up material for robot, and max robot = 4
  (bind _returnvalue (`GameplayStatics.GetActorOfClass` "/Game/Game/Blueprints/BP_ThirdPersonCharacter.BP_ThirdPersonCharacter_C"))
  (if (<= (+ (`/Game/Game/Blueprints/BP_ThirdPersonCharacter.nbSbires` _returnvalue) 1) 4)
    (set `/Game/Game/Blueprints/BP_ThirdPersonCharacter.nbSbires` (+ (`/Game/Game/Blueprints/BP_ThirdPersonCharacter.nbSbires` _returnvalue) 1) _returnvalue)
    (set `/Game/Game/Blueprints/Health/HealthComponent.isPlayer` false (`self.HealthComponent`))
    (bind _nbsbires (`/Game/Game/Blueprints/BP_ThirdPersonCharacter.nbSbires` _returnvalue))
    (if (== _nbsbires 1)
      (`PrimitiveComponent.SetMaterial` _mesh 0 "/Game/Game/Blueprints/Material/blue.blue")
      (goto _label)
      (elif (== _nbsbires 2)
        (`PrimitiveComponent.SetMaterial` _mesh 0 "/Game/Game/Blueprints/Material/purple.purple")
        (goto _label)
        (elif (== _nbsbires 3)
          (`PrimitiveComponent.SetMaterial` _mesh 0 "/Game/Game/Blueprints/Material/green.green")
          (goto _label)
          (else
            (goto _label)))))))

(event `LevelUpSkill`
  (params (skill_Id :type Integer))
  (bind _skills (`self.Skills`))
  (bind _skills_2 (`self.Skills`))
  (bind _skills_3 (`self.Skills`))
  (switch `int` skill_Id
    (:`0`
      (bind _increased (`/Game/Game/Blueprints/Sbire/Skills.Increase` _skills (`/Game/Game/Blueprints/Sbire/Skills.HealthLevel` _skills)))
      (bind _output_get (set `/Game/Game/Blueprints/Sbire/Skills.HealthLevel` _increased _skills))
      (`KismetSystemLibrary.PrintString` (`KismetStringLibrary.Conv_IntToString` _output_get)))
    (:`1`
      (bind _increased_2 (`/Game/Game/Blueprints/Sbire/Skills.Increase` _skills_2 (`/Game/Game/Blueprints/Sbire/Skills.SpeedLevel` _skills_2)))
      (bind _output_get_2 (set `/Game/Game/Blueprints/Sbire/Skills.SpeedLevel` _increased_2 _skills_2))
      (`KismetSystemLibrary.PrintString` (`KismetStringLibrary.Conv_IntToString` _output_get_2)))
    (:`2`
      (bind _increased_3 (`/Game/Game/Blueprints/Sbire/Skills.Increase` _skills_3 (`/Game/Game/Blueprints/Sbire/Skills.DamageLevel` _skills_3)))
      (bind _output_get_3 (set `/Game/Game/Blueprints/Sbire/Skills.DamageLevel` _increased_3 _skills_3))
      (`KismetSystemLibrary.PrintString` (`KismetStringLibrary.Conv_IntToString` _output_get_3)))))

(fn `UserConstructionScript`)