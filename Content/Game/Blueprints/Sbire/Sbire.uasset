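; Sbire is a robot actor that tracks the third-person character's target position while facing the player camera.
; Every tick it rotates toward the camera manager's location, then looks up BP_ThirdPersonCharacter and reads its TargetPosition.
; It moves directly to that position with a fixed X offset and Z flattened to zero, without sweep.
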(event `self.ReceiveTick`
  (params (DeltaSeconds :type "Float (single-precision)"))
  ;[1 1 1] robots rotation
  (`self.K2_SetActorRotation` (`KismetMathLibrary.FindLookAtRotation` (`self.K2_GetActorLocation`) (`SceneComponent.K2_GetComponentLocation` (`Actor.RootComponent` (`GameplayStatics.GetPlayerCameraManager` 0)))))
  (bind _returnvalue (`GameplayStatics.GetActorOfClass` "/Game/Game/Blueprints/BP_ThirdPersonCharacter.BP_ThirdPersonCharacter_C"))
  (`self.K2_SetActorLocation` (* (+ (`/Game/Game/Blueprints/BP_ThirdPersonCharacter.Target Position` _returnvalue) (-150.0 0.0 0.0)) (1.0 1.0 0.0))))

(fn `UserConstructionScript`)